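; BP_ShootingPost is a shooting post actor that shows a camera view of its assigned Target while the player overlaps it.
; On player overlap, it assigns the TargetCameraView texture to the SceneCaptureComponent2D found on Target and prints a debug message naming that Target.
; When the player leaves, it clears that capture's texture target, so only an occupied post feeds the view.
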(event EventBeginPlay)

(event Collision|EventActorBeginOverlap
  (params (OtherActor :type Actor%20Object%20Reference))
  (bind _target (Variables|Default|GetTarget))
  (if (== OtherActor (Game|GetPlayerCharacter 0))
    (Variables|/Script/Engine.SceneCaptureComponent2D|SetTextureTarget (Actor|GetComponentbyClass _target "/Script/Engine.SceneCaptureComponent2D") "/Game/_MyAssets/HUD/TargetCameraView.TargetCameraView")
    (Development|PrintString (Utilities|String|Append "player enter " (Utilities|GetDisplayName _target)))))

(event EventTick
  (params (DeltaSeconds :type Float%20%28single-precision%29)))

(event Collision|EventActorEndOverlap
  (params (OtherActor :type Actor%20Object%20Reference))
  (if (== OtherActor (Game|GetPlayerCharacter 0))
    (Variables|/Script/Engine.SceneCaptureComponent2D|SetTextureTarget (Actor|GetComponentbyClass (Variables|Default|GetTarget) "/Script/Engine.SceneCaptureComponent2D") 0)))

(fn ConstructionScript)