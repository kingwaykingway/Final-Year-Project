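; BP_SpawningPoint is a placeable spawn marker that creates an actor of a configurable class at its own transform.
; It can spawn on BeginPlay via the SpawnAtStart flag, or whenever SpawnObject is called.
; Spawned Weapon subclasses get physics simulation and the Pickup collision profile on their skeletal mesh, with the laser pointer switched off, so they rest in the world as pickups.
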(event EventBeginPlay
  (if (Variables|Default|GetSpawn%20at%20Start)
    (CallFunction|SpawnObject)))

(event Collision|EventActorBeginOverlap
  (params (OtherActor :type Actor%20Object%20Reference)))

(event EventTick
  (params (DeltaSeconds :type Float%20%28single-precision%29)))

(fn ConstructionScript)

(fn SpawnObject
  (bind _object_to_spawn (Variables|Default|GetObject%20To%20Spawn))
  (bind _returnvalue (Game|SpawnActorfromClass _object_to_spawn (Transformation|GetActorTransform) "Undefined" 0 0))
  (if (Utilities|ClassIsChildOf _object_to_spawn "/Script/TPS.Weapon")
    (bind _asweapon (Utilities|Casting|CastToWeapon _returnvalue))
    (Physics|SetSimulatePhysics (Actor|GetComponentbyClass _asweapon "/Script/Engine.SkeletalMeshComponent") true)
    (Collision|SetCollisionProfileName (Actor|GetComponentbyClass _asweapon "/Script/Engine.SkeletalMeshComponent") "Pickup" :!class /Script/Engine.PrimitiveComponent)
    (Class|Weapon|AimLazerPointer _asweapon false)))