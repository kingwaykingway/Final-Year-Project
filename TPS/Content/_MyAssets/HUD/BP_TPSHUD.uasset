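; Third-person shooter HUD that adds the HUD widget and draws full-screen scope overlays for scoped weapons.
; BeginPlay caches the player character and animator, then maps weapon classes to dynamic reticle materials.
; Tick switches scope opacity on once aiming outlasts the weapon's delay without reloading or swapping, hiding gun and body from the owner.
; DrawHUD feeds that opacity into the equipped weapon's material and draws it.
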(event EventBeginPlay
  (Utilities|FlowControl|Sequence
    (:then_0
      (bind _asue_4asp_character (Utilities|Casting|CastToUe4ASP_Character (Game|GetPlayerCharacter (Game|GetPlayerController 0))))
      (bind _output_get (Variables|Reference|SetPlayer%20Character _asue_4asp_character))
      (Variables|Reference|SetPlayer%20Character%20Animator (Variables|/Game/AnimStarterPack/Ue4ASP_Character.Ue4ASP_Character_C|GetAnim _output_get)))
    (:then_1
      (bind _returnvalue (UserInterface|CreateWidget "/Game/_MyAssets/HUD/HUDWidget.HUDWidget_C" (Game|Player|GetOwningPlayerController)))
      (UserInterface|Viewport|AddtoViewport _returnvalue 0))
    (:then_2
      (Utilities|FlowControl|Sequence
        (:then_0
          (bind _returnvalue_2 (Rendering|Material|CreateDynamicMaterialInstance "/Game/_MyAssets/ScopeAndCrosshair/M_SniperReticle_3.M_SniperReticle_3" "None" :!class /Script/Engine.KismetMaterialLibrary)))
        (:then_1
          (bind _returnvalue_3 (Rendering|Material|CreateDynamicMaterialInstance "/Game/_MyAssets/ScopeAndCrosshair/M_SniperReticle_4.M_SniperReticle_4" "None" :!class /Script/Engine.KismetMaterialLibrary)))
        (:then_2
          (bind _returnvalue_4 (Rendering|Material|CreateDynamicMaterialInstance "/Game/_MyAssets/ScopeAndCrosshair/M_SniperReticle_5.M_SniperReticle_5" "None" :!class /Script/Engine.KismetMaterialLibrary)))
        (:then_3
          (bind _returnvalue_5 (Rendering|Material|CreateDynamicMaterialInstance "/Game/_MyAssets/ScopeAndCrosshair/M_SniperReticle_6.M_SniperReticle_6" "None" :!class /Script/Engine.KismetMaterialLibrary)))
        (:then_4
          (bind _returnvalue_6 (Rendering|Material|CreateDynamicMaterialInstance "/Game/_MyAssets/ScopeAndCrosshair/M_SniperReticle_7.M_SniperReticle_7" "None" :!class /Script/Engine.KismetMaterialLibrary)))))
    (:then_3
      (Variables|Reference|SetScopeMaterials (Utilities|Map|MakeMap "/Game/_MyAssets/BP_Weapons/BP_Dark_SniperRifle.BP_Dark_SniperRifle_C" _returnvalue_2 "/Game/_MyAssets/BP_Weapons/BP_Light_SniperRifle.BP_Light_SniperRifle_C" _returnvalue_3 "/Game/_MyAssets/BP_Weapons/BP_Dark_AssaultRifle.BP_Dark_AssaultRifle_C" _returnvalue_4 "/Game/_MyAssets/BP_Weapons/BP_Light_GrenadeLauncher.BP_Light_GrenadeLauncher_C" _returnvalue_5 "/Game/_MyAssets/BP_Weapons/BP_Light_RocketLauncher.BP_Light_RocketLauncher_C" _returnvalue_6)))))

(event Collision|EventActorBeginOverlap
  (params (OtherActor :type Actor%20Object%20Reference)))

(event EventTick
  (params (DeltaSeconds :type Float%20%28single-precision%29))
  (bind _player_character (Variables|Reference|GetPlayer%20Character))
  (bind _equipped_weapon (Variables|/Game/AnimStarterPack/Ue4ASP_Character.Ue4ASP_Character_C|GetEquipped%20Weapon _player_character))
  (bind _anim (Variables|/Game/AnimStarterPack/Ue4ASP_Character.Ue4ASP_Character_C|GetAnim _player_character))
  (bind _aimingdelay (Variables|/Script/TPS.Weapon|GetAimingDelay _equipped_weapon))
  (Utilities|IsValid (Variables|Reference|GetPlayer%20Character%20Animator)
    (:Is%20Valid
      (if (Math|Boolean|ANDBoolean (Variables|/Game/AnimStarterPack/UE4ASP_HeroTPP_AnimBlueprint.UE4ASP_HeroTPP_AnimBlueprint_C|GetAiming (Variables|Reference|GetPlayer%20Character%20Animator)) (not (Variables|/Game/AnimStarterPack/UE4ASP_HeroTPP_AnimBlueprint.UE4ASP_HeroTPP_AnimBlueprint_C|GetReloading (Variables|Reference|GetPlayer%20Character%20Animator))) (not (Variables|/Game/AnimStarterPack/UE4ASP_HeroTPP_AnimBlueprint.UE4ASP_HeroTPP_AnimBlueprint_C|GetSwapping%20Weapon (Variables|Reference|GetPlayer%20Character%20Animator))))
        (Variables|Default|SetAimingDelayTimer (Math|Float|Clamp(Float) (+ DeltaSeconds (Variables|Default|GetAimingDelayTimer)) 0.0 _aimingdelay))
        (else
          (Variables|Default|SetAimingDelayTimer 0.0))))
    (:Is%20Not%20Valid
      (Utilities|FlowControl|DoOnce false
        (:Completed
          (Variables|Reference|SetPlayer%20Character%20Animator _anim)))))
  (bind _output_get (Variables|Default|SetScopeOpacity (Math|Float|SelectFloat 1.0 0.0 (Math|Boolean|ANDBoolean (>= (Variables|Default|GetAimingDelayTimer) _aimingdelay) (Utilities|Enum|Equal(Enum) (Variables|/Script/TPS.Weapon|GetAiming_TargetingTool _equipped_weapon) "TargetingTool_Scope") (not (Variables|/Game/AnimStarterPack/UE4ASP_HeroTPP_AnimBlueprint.UE4ASP_HeroTPP_AnimBlueprint_C|GetReloading _anim)) (not (Variables|/Game/AnimStarterPack/UE4ASP_HeroTPP_AnimBlueprint.UE4ASP_HeroTPP_AnimBlueprint_C|GetSwapping%20Weapon _anim))))))
  (Class|PrimitiveComponent|SetOwnerNoSee (Variables|/Script/TPS.Weapon|GetGunMesh (Variables|/Game/AnimStarterPack/Ue4ASP_Character.Ue4ASP_Character_C|GetEquipped%20Weapon (Variables|Reference|GetPlayer%20Character))) (>= _output_get 1.0)))

(event EventDrawHUD
  (params (SizeX :type Integer) (SizeY :type Integer))
  (bind _player_character (Variables|Reference|GetPlayer%20Character))
  (bind _scopematerials (Variables|Reference|GetScopeMaterials))
  (bind _equipped_weapon (Variables|/Game/AnimStarterPack/Ue4ASP_Character.Ue4ASP_Character_C|GetEquipped%20Weapon _player_character))
  (bind _returnvalue (Utilities|GetClass _equipped_weapon))
  (bind (_value _returnvalue_2) (Utilities|Map|Find _scopematerials _returnvalue))
  (if _returnvalue_2
    (Utilities|FlowControl|Sequence
      (:then_1
        (Rendering|Material|SetScalarParameterValue _value "ScopeOpacity" (Variables|Default|GetScopeOpacity) :!class /Script/Engine.MaterialInstanceDynamic))
      (:then_2
        (Canvas|DrawMaterial _value 0.0 0.0 (Math|Conversions|ToFloat(Integer) SizeX) (Math|Conversions|ToFloat(Integer) SizeY) 0.0 0.0 1.0 1.0)))))

(fn ConstructionScript)

(fn SelectScopeMat)