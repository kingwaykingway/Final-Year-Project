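; Rocket launcher weapon that fires a laser-guided BP_Missile_Dark.
; Fire spawns the missile at the muzzle offset, stores it as LinkedMissile, sets its speed and default target, and hides the dummy rocket, which reloads show again.
; AimLazerPointer traces along the beam and retargets the live missile to the hit point.
; Beam color shows red when guiding, yellow when the trace misses, green with no missile in flight.
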(event EventBeginPlay)

(event Collision|EventActorBeginOverlap
  (params (OtherActor :type Actor%20Object%20Reference)))

(event EventTick
  (params (DeltaSeconds :type Float%20%28single-precision%29)))

(event EventReloadHip
  ;[1 1 1] Reloadings
  (Rendering|SetVisibility (Variables|Default|GetDummy%20Ammo) true false)
  (Components|Animation|PlayAnimation (Variables|Default|GetSkeletalMesh) "/Game/SciFiWeapDark/Weapons/Anims/Reload_RocketLauncher_W.Reload_RocketLauncher_W" false))

(event EventFire
  ;[1 1 1] Fire
  (Components|Animation|PlayAnimation (Variables|Default|GetSkeletalMesh) "/Game/SciFiWeapDark/Weapons/Anims/Fire_RocketLauncher_W.Fire_RocketLauncher_W" false)
  (Variables|Default|SetRemainingAmmo (- (Variables|Default|GetRemainingAmmo) 1))
  (Rendering|SetVisibility (Variables|Default|GetDummy%20Ammo) false false)
  (bind _returnvalue (Game|SpawnActorfromClass "/Game/_MyAssets/BP_Weapons/Projectiles/BP_Missile_Dark.BP_Missile_Dark_C" (Math|Transform|MakeTransform (+ (Transformation|GetWorldLocation (Variables|Default|GetRoot)) (Math|Transform|TransformLocation (Math|Conversions|ToTransform(Rotator) (Transformation|GetActorRotation)) (Variables|Default|GetMuzzleOffset))) (Transformation|GetActorRotation)) "AlwaysSpawn" self (Variables|Default|GetInstigator)))
  (bind _output_get (Variables|Default|SetLinked%20Missile _returnvalue))
  (Utilities|FlowControl|Sequence
    (:then_0
      (bind _output_get_2 (Variables|/Script/Engine.ProjectileMovementComponent|SetInitialSpeed (Variables|/Script/TPS.Projectile|GetProjectileMovementComponent _output_get) (Variables|Default|GetMuzzleVelocity)))
      (Variables|/Script/Engine.ProjectileMovementComponent|SetMaxSpeed (Variables|/Script/TPS.Projectile|GetProjectileMovementComponent _output_get) _output_get_2))
    (:then_1
      (Variables|/Game/_MyAssets/BP_Weapons/Projectiles/BP_Abstract_Rocket.BP_Abstract_Rocket_C|SetTarget%20Location _output_get (* (Transformation|GetActorForwardVector _output_get) (Variables|Default|GetRange))))))

(event EventReloadIronsights
  ;[1 1 1] Reloadings
  (Rendering|SetVisibility (Variables|Default|GetDummy%20Ammo) true false)
  (Components|Animation|PlayAnimation (Variables|Default|GetSkeletalMesh) "/Game/SciFiWeapDark/Weapons/Anims/Reload_RocketLauncher_W.Reload_RocketLauncher_W" false))

(event EventReloadProne
  ;[1 1 1] Reloadings
  (Rendering|SetVisibility (Variables|Default|GetDummy%20Ammo) true false)
  (Components|Animation|PlayAnimation (Variables|Default|GetSkeletalMesh) "/Game/SciFiWeapDark/Weapons/Anims/Reload_RocketLauncher_W.Reload_RocketLauncher_W" false))

(event EventAimLazerPointer
  (params (activate :type Boolean))
  (bind _lazer_pointer (Variables|Default|GetLazer%20Pointer))
  (bind _linked_missile (Variables|Default|GetLinked%20Missile))
  (bind _lazer_pointer_2 (Variables|Default|GetLazer%20Pointer))
  (bind _lazer_pointer_3 (Variables|Default|GetLazer%20Pointer))
  (bind _returnvalue (Transformation|GetWorldLocation _lazer_pointer_3))
  ;[1 1 1] Target the missile
  (Rendering|SetVisibility (Variables|Default|GetLazer%20Pointer) activate false)
  (if activate
    (Class|ParticleSystemComponent|SetBeamSourcePoint _lazer_pointer_3 0 _returnvalue)
    (bind (_outhit _returnvalue_2) (Collision|LineTraceByChannel _returnvalue (+ _returnvalue (* (Math|Vector|GetForwardVector _lazer_pointer_3) (Variables|Default|GetRange))) (Utilities|Enum|LiteralenumETraceTypeQuery "TraceTypeQuery1") false 0 "None"))
    (if _returnvalue_2
      (Class|ParticleSystemComponent|SetBeamTargetPoint _lazer_pointer_2 0 (.Location (Collision|BreakHitResult _outhit)))
      (Utilities|IsValid _linked_missile
        (:Is%20Valid
          (Variables|/Game/_MyAssets/BP_Weapons/Projectiles/BP_Abstract_Rocket.BP_Abstract_Rocket_C|SetTarget%20Location _linked_missile (.Location (Collision|BreakHitResult _outhit)))
          (Effects|Components|ParticleSystem|SetColorParameter _lazer_pointer "Color" "(R=1.000000,G=0.000000,B=0.000000,A=1.000000)")
          (Variables|Default|SetIs%20Target%20Lost false))
        (:Is%20Not%20Valid
          (Effects|Components|ParticleSystem|SetColorParameter _lazer_pointer "Color" "(R=0.000000,G=1.000000,B=0.000000,A=1.000000)" :!label _label)
          (Variables|Default|SetIs%20Target%20Lost false)))
      (else
        (Class|ParticleSystemComponent|SetBeamTargetPoint _lazer_pointer_2 0 (.TraceEnd (Collision|BreakHitResult _outhit)))
        (Utilities|IsValid _linked_missile
          (:Is%20Valid
            (Effects|Components|ParticleSystem|SetColorParameter _lazer_pointer "Color" "(R=1.000000,G=1.000000,B=0.000000,A=1.000000)")
            (Variables|Default|SetIs%20Target%20Lost true))
          (:Is%20Not%20Valid
            (goto _label)))))))

(event EventBeginPlayChild
  (Rendering|SetVisibility (Variables|Default|GetDummy%20Ammo) true false))

(fn ConstructionScript)