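; Dark sniper rifle weapon with a charged shot that spends extra ammo for a larger, higher-impact bullet.
; Tick caps the charge timer by remaining ammo and beeps at each fifth of full charge, gated by a DoOnce.
; Fire converts charge into ammo cost, projectile scale and impact level, while GetRecoil multiplies the parent's recoil by charge.
; Reload events play gun animations for hip, ironsights and prone.
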(event EventBeginPlay)

(event Collision|EventActorBeginOverlap
  (params (OtherActor :type Actor%20Object%20Reference)))

(event EventTick
  (params (DeltaSeconds :type Float%20%28single-precision%29))
  (bind _returnvalue (Math|Float|MakeLiteralFloat 0.01))
  (Utilities|FlowControl|Sequence
    (:then_0
      (Variables|Default|SetFireChargingTimer (Math|Float|Clamp(Float) (Variables|Default|GetFireChargingTimer) 0.0 (* (- (Variables|Default|GetRemainingAmmo) 1) (/ (Variables|Default|GetMaxFireCharging) (Math|Conversions|ToFloat(Integer) (- (Variables|Default|GetMagazineSize) 1)))))))
    (:then_1
      ;[1 1 1] Each time the fire charging reaches a fraction, beep once
      (if (> (Variables|Default|GetMaxFireCharging) 0.0)
        (if (Math|Boolean|ORBoolean (Math|Float|NearlyEqual(Float) (/ (Variables|Default|GetFireChargingTimer) (Variables|Default|GetMaxFireCharging)) 0.2 _returnvalue) (Math|Float|NearlyEqual(Float) (/ (Variables|Default|GetFireChargingTimer) (Variables|Default|GetMaxFireCharging)) 0.4 _returnvalue) (Math|Float|NearlyEqual(Float) (/ (Variables|Default|GetFireChargingTimer) (Variables|Default|GetMaxFireCharging)) 0.6 _returnvalue) (Math|Float|NearlyEqual(Float) (/ (Variables|Default|GetFireChargingTimer) (Variables|Default|GetMaxFireCharging)) 0.8 _returnvalue) (Math|Float|NearlyEqual(Float) (/ (Variables|Default|GetFireChargingTimer) (Variables|Default|GetMaxFireCharging)) 1.0 _returnvalue))
          (Utilities|FlowControl|DoOnce false :!label _label
            (:Completed
              (Audio|PlaySoundatLocation "/Engine/EditorSounds/Notifications/CompileStart_Cue.CompileStart_Cue" (Transformation|GetActorLocation) (Transformation|GetActorRotation) 1.0 1.0 0.0 0 0 self)))
          (else
            (goto _label Reset)))))))

(event EventReloadHip
  ;[1 1 1] Reloadings
  (Components|Animation|PlayAnimation (Variables|Default|GetGunMesh) "/Game/SciFiWeapDark/Weapons/Anims/Reload_SniperRifle_Hips_W.Reload_SniperRifle_Hips_W" false))

(event EventFire
  ;[1 1 1] Fire
  (Components|Animation|PlayAnimation (Variables|Default|GetSkeletalMesh) (Variables|Default|GetFiringAnim) false)
  (Variables|Default|SetRemainingAmmo (Math|Integer|Clamp(Integer) (- (Variables|Default|GetRemainingAmmo) (Math|Integer|SelectInt (+ (Math|Float|Floor (* 5 (/ (Variables|Default|GetFireChargingTimer) (Variables|Default|GetMaxFireCharging)))) 1) 1 (> (Variables|Default|GetMaxFireCharging) 0.0))) 0 (Variables|Default|GetMagazineSize)))
  (bind _returnvalue (Game|SpawnActorfromClass "/Game/_MyAssets/BP_Weapons/Projectiles/BP_Bullet_Dark_SniperRifle.BP_Bullet_Dark_SniperRifle_C" (Math|Transform|MakeTransform (+ (Transformation|GetActorLocation) (Math|Transform|TransformLocation (Math|Conversions|ToTransform(Rotator) (Transformation|GetActorRotation)) (Variables|Default|GetMuzzleOffset))) (Transformation|GetActorRotation) (Math|Conversions|ToVector(Float) (+ (/ (Math|Conversions|ToFloat(Integer) (Math|Float|Floor (* 5 (/ (Variables|Default|GetFireChargingTimer) (Variables|Default|GetMaxFireCharging))))) 1e+01) 0.5))) "AlwaysSpawn" self (Variables|Default|GetInstigator)))
  (Utilities|FlowControl|Sequence
    (:then_0
      (bind _output_get (Variables|/Script/Engine.ProjectileMovementComponent|SetInitialSpeed (Variables|/Script/TPS.Projectile|GetProjectileMovementComponent _returnvalue) (Variables|Default|GetMuzzleVelocity)))
      (Variables|/Script/Engine.ProjectileMovementComponent|SetMaxSpeed (Variables|/Script/TPS.Projectile|GetProjectileMovementComponent _returnvalue) _output_get))
    (:then_1
      (Variables|/Script/TPS.Projectile|SetRange _returnvalue (Variables|Default|GetRange))
      (Variables|/Game/_MyAssets/BP_Weapons/Projectiles/BP_Bullet_Dark_SniperRifle.BP_Bullet_Dark_SniperRifle_C|SetImpact%20Level _returnvalue (Math|Float|Floor (* 5 (/ (/ (Variables|Default|GetFireChargingTimer) (Variables|Default|GetMaxFireCharging)) 2.0)))))
    (:then_2
      (Class|Projectile|FireinDirection _returnvalue (Transformation|GetActorForwardVector _returnvalue)))))

(event EventReloadProne
  ;[1 1 1] Reloadings
  (Components|Animation|PlayAnimation (Variables|Default|GetGunMesh) "/Game/SciFiWeapDark/Weapons/Anims/Prone_SniperRifle_Reload_W.Prone_SniperRifle_Reload_W" false))

(event EventReloadIronsights
  ;[1 1 1] Reloadings
  (Components|Animation|PlayAnimation (Variables|Default|GetGunMesh) "/Game/SciFiWeapDark/Weapons/Anims/Reload_SniperRifle_Ironsights_W.Reload_SniperRifle_Ironsights_W" false))

(fn ConstructionScript)

(fn GetRecoil
  (params (aiming :type Boolean))
  (bind _returnvalue (|CallParentFunction aiming))
  (return (* _returnvalue (+ (/ (Variables|Default|GetFireChargingTimer) (Variables|Default|GetMaxFireCharging)) 1.0))))