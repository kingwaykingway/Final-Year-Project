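; Light rocket launcher weapon that fires a BP_Missile_Light, homing on a locked target or aimed straight ahead without one.
; While scoped, AimScope picks "Lockable" actors by angle from forward and advances per-weapon progress on their BP_MissileLockWidget until locked.
; A separate, configurable angle threshold breaks the lock.
; Fire and reload events animate the mesh and toggle the dummy rocket; older laser-guidance code remains disconnected.
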(event EventBeginPlay)

(event Collision|EventActorBeginOverlap
  (params (OtherActor :type Actor%20Object%20Reference)))

(event EventTick
  (params (DeltaSeconds :type Float%20%28single-precision%29)))

(event EventReloadHip
  ;[1 1 1] Reloadings
  (Rendering|SetVisibility (Variables|Default|GetDummy%20Ammo) true false)
  (Components|Animation|PlayAnimation (Variables|Default|GetSkeletalMesh) "/Game/SciFiWeapLight/Weapons/Anims/Reload_RocketLauncher_W.Reload_RocketLauncher_W" false))

(event EventFire
  (bind _locked_target (Variables|Default|GetLocked%20Target))
  ;[1 1 1] Fire
  (Components|Animation|PlayAnimation (Variables|Default|GetSkeletalMesh) "/Game/SciFiWeapLight/Weapons/Anims/Fire_RocketLauncher_W.Fire_RocketLauncher_W" false)
  (Variables|Default|SetRemainingAmmo (- (Variables|Default|GetRemainingAmmo) 1))
  (Rendering|SetVisibility (Variables|Default|GetDummy%20Ammo) false false)
  (bind _returnvalue (Game|SpawnActorfromClass "/Game/_MyAssets/BP_Weapons/Projectiles/BP_Missile_Light.BP_Missile_Light_C" (Math|Transform|MakeTransform (+ (Transformation|GetActorLocation) (Math|Transform|TransformLocation (Math|Conversions|ToTransform(Rotator) (Transformation|GetActorRotation)) (Variables|Default|GetMuzzleOffset))) (Transformation|GetActorRotation)) "AlwaysSpawn" self (Variables|Default|GetInstigator)))
  (bind _output_get (Variables|Default|SetLinked%20Missile _returnvalue))
  (Utilities|FlowControl|Sequence
    (:then_0
      (bind _output_get_2 (Variables|/Script/Engine.ProjectileMovementComponent|SetInitialSpeed (Variables|/Script/TPS.Projectile|GetProjectileMovementComponent _output_get) (Variables|Default|GetMuzzleVelocity)))
      (Variables|/Script/Engine.ProjectileMovementComponent|SetMaxSpeed (Variables|/Script/TPS.Projectile|GetProjectileMovementComponent _output_get) _output_get_2))
    (:then_1
      (Utilities|IsValid _locked_target
        (:Is%20Valid
          (Variables|/Game/_MyAssets/BP_Weapons/Projectiles/BP_Abstract_Rocket.BP_Abstract_Rocket_C|SetLockedTarget _output_get _locked_target))
        (:Is%20Not%20Valid
          (Variables|/Game/_MyAssets/BP_Weapons/Projectiles/BP_Abstract_Rocket.BP_Abstract_Rocket_C|SetTarget%20Location _output_get (* (Transformation|GetActorForwardVector _output_get) (Variables|Default|GetRange))))))))

(event EventReloadIronsights
  ;[1 1 1] Reloadings
  (Rendering|SetVisibility (Variables|Default|GetDummy%20Ammo) true false)
  (Components|Animation|PlayAnimation (Variables|Default|GetSkeletalMesh) "/Game/SciFiWeapLight/Weapons/Anims/Reload_RocketLauncher_W.Reload_RocketLauncher_W" false))

(event EventReloadProne
  ;[1 1 1] Reloadings
  (Rendering|SetVisibility (Variables|Default|GetDummy%20Ammo) true false)
  (Components|Animation|PlayAnimation (Variables|Default|GetSkeletalMesh) "/Game/SciFiWeapLight/Weapons/Anims/Reload_RocketLauncher_W.Reload_RocketLauncher_W" false))

(event EventAimScope
  (params (activate :type Boolean))
  (|CallParentFunction activate)
  (Utilities|FlowControl|Sequence
    (:then_0
      (if activate
        (Utilities|FlowControl|DoOnce false :!label _label
          (:Completed
            (bind _outactors (Actor|GetAllActorswithTag "Lockable"))
            (for _array_element _outactors
              (bind _asbp_missile_lock_widget (Utilities|Casting|CastToBP_MissileLockWidget (UserInterface|GetUserWidgetObject (Actor|GetComponentbyClass _array_element "/Script/UMG.WidgetComponent"))))
              (Variables|/Game/_MyAssets/ScopeAndCrosshair/BP_MissileLockWidget.BP_MissileLockWidget_C|SetIs%20Activated _asbp_missile_lock_widget true)
              (Variables|Default|SetMin%20Target%20Angle (Variables|Default|GetLocking%20Critical%20Angle)))))
        (else
          (goto _label Reset))))
    (:then_1
      (if activate
        (goto _label_2 Reset)
        (else
          (Utilities|FlowControl|DoOnce false :!label _label_2
            (:Completed
              (bind _outactors_2 (Actor|GetAllActorswithTag "Lockable"))
              (for _array_element_2 _outactors_2
                (bind _asbp_missile_lock_widget_2 (Utilities|Casting|CastToBP_MissileLockWidget (UserInterface|GetUserWidgetObject (Actor|GetComponentbyClass _array_element_2 "/Script/UMG.WidgetComponent"))))
                (Variables|/Game/_MyAssets/ScopeAndCrosshair/BP_MissileLockWidget.BP_MissileLockWidget_C|SetIs%20Activated _asbp_missile_lock_widget_2 false)
                (Variables|Default|SetMin%20Target%20Angle (Variables|Default|GetLocking%20Critical%20Angle)))
              (Variables|Default|SetLocking%20Target 0)
              (Variables|Default|SetLocked%20Target 0))))))
    (:then_2
      (if activate
        (bind _outactors_3 (Actor|GetAllActorswithTag "Lockable"))
        (Utilities|FlowControl|Sequence
          (:then_0
            (if (not (Utilities|IsValid (Variables|Default|GetLocked%20Target)))
              (for _array_element_3 _outactors_3
                (bind _returnvalue (Class|TPSFunctionLibrary|AngleBetweenVectors (Transformation|GetActorForwardVector) (- (Transformation|GetActorLocation _array_element_3) (Transformation|GetActorLocation))))
                (if (<= _returnvalue (Variables|Default|GetLocking%20Critical%20Angle))
                  (if (< _returnvalue (Variables|Default|GetMin%20Target%20Angle))
                    (Variables|Default|SetLocking%20Target _array_element_3)
                    (else
                      (Variables|Default|SetMin%20Target%20Angle _returnvalue)))
                  (else
                    (bind _asbp_missile_lock_widget_3 (Utilities|Casting|CastToBP_MissileLockWidget (UserInterface|GetUserWidgetObject (Actor|GetComponentbyClass _array_element_3 "/Script/UMG.WidgetComponent"))))
                    (Default|Unlock _asbp_missile_lock_widget_3 self))))
              (Variables|Default|SetMin%20Target%20Angle (Variables|Default|GetLocking%20Critical%20Angle))
              (else
                (bind _returnvalue_2 (Class|TPSFunctionLibrary|AngleBetweenVectors (Transformation|GetActorForwardVector) (- (Transformation|GetActorLocation (Variables|Default|GetLocked%20Target)) (Transformation|GetActorLocation))))
                (if (>= _returnvalue_2 (Variables|Default|GetUnlocking%20Critical%20Angle))
                  (bind _asbp_missile_lock_widget_4 (Utilities|Casting|CastToBP_MissileLockWidget (UserInterface|GetUserWidgetObject (Actor|GetComponentbyClass (Variables|Default|GetLocked%20Target) "/Script/UMG.WidgetComponent"))))
                  (Default|Unlock _asbp_missile_lock_widget_4 self)
                  (Variables|Default|SetLocked%20Target 0)))))
          (:then_1
            (for _array_element_4 _outactors_3
              (bind _asbp_missile_lock_widget_5 (Utilities|Casting|CastToBP_MissileLockWidget (UserInterface|GetUserWidgetObject (Actor|GetComponentbyClass _array_element_4 "/Script/UMG.WidgetComponent"))))
              (if (== _array_element_4 (Variables|Default|GetLocking%20Target))
                (Default|Lock _asbp_missile_lock_widget_5 self (* (Utilities|Time|GetWorldDeltaSeconds) (Variables|Default|GetLocking%20Rate)))
                (if (and (>= (.Value (Utilities|Map|Find (Variables|/Game/_MyAssets/ScopeAndCrosshair/BP_MissileLockWidget.BP_MissileLockWidget_C|GetLockingProgress _asbp_missile_lock_widget_5) self)) 1.0) (.ReturnValue (Utilities|Map|Find (Variables|/Game/_MyAssets/ScopeAndCrosshair/BP_MissileLockWidget.BP_MissileLockWidget_C|GetLockingProgress _asbp_missile_lock_widget_5) self)))
                  (Variables|Default|SetLocked%20Target (Variables|Default|GetLocking%20Target)))
                (else
                  (Default|Unlock _asbp_missile_lock_widget_5))))))))))

(event EventUnaim
  (|CallParentFunction)
  (Class|Weapon|AimScope false))

(fn ConstructionScript)

(fn VisualizeMissileLockingWidgets)