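; BP_Dark_Shotgun is a shotgun weapon Blueprint that appears to extend a parent weapon class.
; On child begin play it gives a valid crosshair a circular sight pattern.
; Hip, ironsights and prone reloads all play the same shotgun reload animation on the skeletal mesh.
; Its multi-projectile fire logic, which scatters BP_Bullet_Dark_Shotgun spawns with a random circular spread, is disconnected and never runs here.
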(event EventBeginPlay)

(event Collision|EventActorBeginOverlap
  (params (OtherActor :type Actor%20Object%20Reference)))

(event EventTick
  (params (DeltaSeconds :type Float%20%28single-precision%29)))

(event EventReloadHip
  ;[1 1 1] Reloadings
  (Components|Animation|PlayAnimation (Variables|Default|GetSkeletalMesh) "/Game/SciFiWeapDark/Weapons/Anims/Reload_Shotgun_W.Reload_Shotgun_W" false))

(event EventReloadProne
  ;[1 1 1] Reloadings
  (Components|Animation|PlayAnimation (Variables|Default|GetSkeletalMesh) "/Game/SciFiWeapDark/Weapons/Anims/Reload_Shotgun_W.Reload_Shotgun_W" false))

(event EventReloadIronsights
  ;[1 1 1] Reloadings
  (Components|Animation|PlayAnimation (Variables|Default|GetSkeletalMesh) "/Game/SciFiWeapDark/Weapons/Anims/Reload_Shotgun_W.Reload_Shotgun_W" false))

(event EventBeginPlayChild
  (bind _crosshair (Variables|Default|GetCrosshair))
  (Utilities|IsValid _crosshair
    (:Is%20Valid
      (Variables|/Script/TPS.CrosshairWidget|SetSightPattern _crosshair "SightPattern_Circle"))))

(fn ConstructionScript)