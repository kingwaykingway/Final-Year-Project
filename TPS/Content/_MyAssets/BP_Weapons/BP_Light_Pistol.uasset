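; Light pistol weapon Blueprint that sets a dot crosshair and fires a charge-scaled projectile.
; Fire plays the firing animation, deducts ammo and spawns BP_Bullet_Light_Pistol at the muzzle offset with the weapon's velocity and range.
; Charge ratio raises ammo cost, bullet scale and the parent's recoil, up to double for scale and recoil at full charge.
; Hip, ironsights and prone reloads share one animation.
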(event EventBeginPlay)

(event Collision|EventActorBeginOverlap
  (params (OtherActor :type Actor%20Object%20Reference)))

(event EventTick
  (params (DeltaSeconds :type Float%20%28single-precision%29)))

(event EventReloadHip
  ;[1 1 1] Reloadings
  (Components|Animation|PlayAnimation (Variables|Default|GetSkeletalMesh) "/Game/SciFiWeapLight/Weapons/Anims/Reload_Pistol_W.Reload_Pistol_W" false))

(event EventBeginPlayChild
  (bind _crosshair (Variables|Default|GetCrosshair))
  (Utilities|IsValid _crosshair
    (:Is%20Valid
      (Variables|/Script/TPS.CrosshairWidget|SetSightPattern _crosshair "SightPattern_Dot"))))

(event EventReloadIronsights
  ;[1 1 1] Reloadings
  (Components|Animation|PlayAnimation (Variables|Default|GetSkeletalMesh) "/Game/SciFiWeapLight/Weapons/Anims/Reload_Pistol_W.Reload_Pistol_W" false))

(event EventReloadProne
  ;[1 1 1] Reloadings
  (Components|Animation|PlayAnimation (Variables|Default|GetSkeletalMesh) "/Game/SciFiWeapLight/Weapons/Anims/Reload_Pistol_W.Reload_Pistol_W" false))

(event EventFire
  (bind (_x _y) (Math|Vector2D|BreakVector2D))
  (bind _returnvalue (Transformation|GetActorRotation))
  (bind (_roll _pitch _yaw) (Math|Rotator|BreakRotator _returnvalue))
  ;[1 1 1] Fire
  (Components|Animation|PlayAnimation (Variables|Default|GetSkeletalMesh) (Variables|Default|GetFiringAnim) false)
  (Variables|Default|SetRemainingAmmo (Math|Integer|Clamp(Integer) (- (Variables|Default|GetRemainingAmmo) (Math|Integer|SelectInt (+ (Math|Float|Floor (* 4 (/ (Variables|Default|GetFireChargingTimer) (Variables|Default|GetMaxFireCharging)))) 1) 1 (> (Variables|Default|GetMaxFireCharging) 0.0))) 0 (Variables|Default|GetMagazineSize)))
  (Class|TPSFunctionLibrary|CircleDistributionRandom (Variables|Default|GetSpread) (Variables|Default|GetSpreadWithNormalDistribution))
  (bind _returnvalue_2 (Game|SpawnActorfromClass "/Game/_MyAssets/BP_Weapons/Projectiles/BP_Bullet_Light_Pistol.BP_Bullet_Light_Pistol_C" (Math|Transform|MakeTransform (+ (Transformation|GetActorLocation) (Math|Transform|TransformLocation (Math|Conversions|ToTransform(Rotator) (Transformation|GetActorRotation)) (Variables|Default|GetMuzzleOffset))) (Math|Rotator|MakeRotator _roll (+ _pitch _x) (+ _yaw _y)) (Math|Conversions|ToVector(Float) (+ (/ (Variables|Default|GetFireChargingTimer) (Variables|Default|GetMaxFireCharging)) 1.0))) "AlwaysSpawn" self (Variables|Default|GetInstigator)))
  (Utilities|FlowControl|Sequence
    (:then_0
      (bind _output_get (Variables|/Script/Engine.ProjectileMovementComponent|SetInitialSpeed (Variables|/Script/TPS.Projectile|GetProjectileMovementComponent _returnvalue_2) (Variables|Default|GetMuzzleVelocity)))
      (Variables|/Script/Engine.ProjectileMovementComponent|SetMaxSpeed (Variables|/Script/TPS.Projectile|GetProjectileMovementComponent _returnvalue_2) _output_get))
    (:then_1
      (Variables|/Script/TPS.Projectile|SetRange _returnvalue_2 (Variables|Default|GetRange)))
    (:then_2
      (Class|Projectile|FireinDirection _returnvalue_2 (Transformation|GetActorForwardVector _returnvalue_2)))))

(fn ConstructionScript)

(fn GetRecoil
  (params (aiming :type Boolean))
  (bind _returnvalue (|CallParentFunction aiming))
  (return (* _returnvalue (+ (/ (Variables|Default|GetFireChargingTimer) (Variables|Default|GetMaxFireCharging)) 1.0))))