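; Light sniper rifle weapon Blueprint that supplies the gun's own reload animations.
; Three reload events, for hip, ironsights and prone, each play the matching non-looping animation on GunMesh.
; An expired scope-aiming override that blends the camera view target between the rifle and the player character remains in the graph but never runs.
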(event EventBeginPlay)

(event Collision|EventActorBeginOverlap
  (params (OtherActor :type Actor%20Object%20Reference)))

(event EventTick
  (params (DeltaSeconds :type Float%20%28single-precision%29)))

(event EventReloadHip
  ;[1 1 1] Reloadings
  (Components|Animation|PlayAnimation (Variables|Default|GetGunMesh) "/Game/SciFiWeapLight/Weapons/Anims/Reload_SniperRifle_Hips_W.Reload_SniperRifle_Hips_W" false))

(event EventReloadProne
  ;[1 1 1] Reloadings
  (Components|Animation|PlayAnimation (Variables|Default|GetGunMesh) "/Game/SciFiWeapLight/Weapons/Anims/Prone_Reload_SniperRifle_W.Prone_Reload_SniperRifle_W" false))

(event EventReloadIronsights
  ;[1 1 1] Reloadings
  (Components|Animation|PlayAnimation (Variables|Default|GetGunMesh) "/Game/SciFiWeapLight/Weapons/Anims/Reload_SniperRifle_Ironsights_W.Reload_SniperRifle_Ironsights_W" false))

(fn ConstructionScript)