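; Dark Pistol bullet projectile Blueprint that handles its impact effects and cleanup.
; On Hit, it spawns a small dark metal impact emitter aligned to the surface normal, plays an attenuated rifle impact sound, then destroys itself.
; The construction script calls its parent, then sets HitEmitter and HitSound (a shotgun impact cue).
; The Hit event uses its own hard-coded assets instead of those variables.
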(event EventBeginPlay
  (|CallParentFunction) ; 此节点被禁用，将不会被调用。\n从引脚连出引线来编译功能。
)

(event Collision|EventActorBeginOverlap
  (params (OtherActor :type Actor%20Object%20Reference))
  (|CallParentFunction OtherActor) ; 此节点被禁用，将不会被调用。\n从引脚连出引线来编译功能。
)

(event EventTick
  (params (DeltaSeconds :type Float%20%28single-precision%29))
  (|CallParentFunction DeltaSeconds) ; 此节点被禁用，将不会被调用。\n从引脚连出引线来编译功能。
)

(event Collision|EventHit
  (params (MyComp :type Primitive%20Component%20Object%20Reference) (Other :type Actor%20Object%20Reference) (OtherComp :type Primitive%20Component%20Object%20Reference) (bSelfMoved :type Boolean) (HitLocation :type Vector :default "0, 0, 0") (HitNormal :type Vector :default "0, 0, 0") (NormalImpulse :type Vector :default "0, 0, 0") (Hit :type Hit%20Result%20Structure%20%28by%20ref%29))
  (bind _returnvalue (Math|Conversions|RotationFromXVector HitNormal))
  (Utilities|FlowControl|Sequence
    (:then_0
      (Effects|SpawnEmitteratLocation "/Game/SciFiWeapDark/FX/Particles/P_Impact_Metal_Small_Dark.P_Impact_Metal_Small_Dark" HitLocation _returnvalue))
    (:then_1
      (Audio|PlaySoundatLocation "/Game/SciFiWeapDark/Sound/Rifle/Rifle_ImpactSurface_Cue.Rifle_ImpactSurface_Cue" HitLocation _returnvalue 1.0 1.0 0.0 "/Game/SciFiWeapDark/Sound/Attenuation/ProjectileImpact_att.ProjectileImpact_att" 0 0))
    (:then_2
      (Actor|DestroyActor))))

(fn ConstructionScript
  (|CallParentFunction)
  (Variables|Default|SetHitEmitter "/Game/SciFiWeapDark/FX/Particles/P_Impact_Metal_Small_Dark.P_Impact_Metal_Small_Dark")
  (Variables|Default|SetHitSound "/Game/SciFiWeapDark/Sound/Shotgun/Shotgun_ImpactSurface_Cue.Shotgun_ImpactSurface_Cue"))