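; Sniper rifle HEIAP bullet projectile that penetrates what it hits and bursts into fragments on exit.
; Collider begin overlap spawns impact effect, sound and an entry bullet-hole decal.
; End overlap multi-traces back toward StartLocation to find the exited actor's surface for the exit decal and effect.
; It then fires BP_Frag_Light_HEIAP projectiles from that point, randomly spread around the bullet's heading, and destroys itself.
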(event OnComponentBeginOverlap(Collider)
  (params (OverlappedComponent :type Primitive%20Component%20Object%20Reference) (OtherActor :type Actor%20Object%20Reference) (OtherComp :type Primitive%20Component%20Object%20Reference) (OtherBodyIndex :type Integer) (bFromSweep :type Boolean) (SweepResult :type Hit%20Result%20Structure%20%28by%20ref%29))
  (bind (_bblockinghit _binitialoverlap _time _distance _location _impactpoint _normal) (Collision|BreakHitResult SweepResult))
  (bind _returnvalue (Math|Conversions|RotationFromXVector _normal))
  (Variables|Default|SetIs%20Overlapping true)
  (Utilities|FlowControl|Sequence
    (:then_0
      (Effects|SpawnEmitteratLocation (Variables|Default|GetHitEmitter) _location _returnvalue (Math|Conversions|ToVector(Float) (Variables|Default|GetEmitterScale))))
    (:then_1
      (Audio|PlaySoundatLocation (Variables|Default|GetHitSound) _location _returnvalue 1.0 1.0 0.0 (Variables|Default|GetHitSoundAttenuation) 0 0))
    (:then_2
      (CallFunction|SpawnBulletHoleDecal (+ _location (* (Transformation|GetActorForwardVector) (Variables|/Script/Engine.SphereComponent|GetSphereRadius (Variables|Default|GetCollider)))) _normal))))

(event OnComponentEndOverlap(Collider)
  (params (OverlappedComponent :type Primitive%20Component%20Object%20Reference) (OtherActor :type Actor%20Object%20Reference) (OtherComp :type Primitive%20Component%20Object%20Reference) (OtherBodyIndex :type Integer))
  (bind _returnvalue (Transformation|GetActorRotation))
  (bind _collider (Variables|Default|GetCollider))
  (bind (_roll _pitch _yaw) (Math|Rotator|BreakRotator _returnvalue))
  (bind _sphereradius (Variables|/Script/Engine.SphereComponent|GetSphereRadius _collider))
  (Variables|Default|SetIs%20Overlapping false)
  (bind _outhits (Collision|MultiLineTraceByChannel (Transformation|GetActorLocation) (Variables|Default|GetStartLocation) "TraceTypeQuery1" false 0 "None"))
  (bind _array_element (Utilities|Array|ForEachLoopwithBreak _outhits :!label _label)
    (:LoopBody
      (if (and (.bBlockingHit (Collision|BreakHitResult _array_element)) (== (.HitActor (Collision|BreakHitResult _array_element)) OtherActor))
        (CallFunction|SpawnBulletHoleDecal (- (+ (.Location (Collision|BreakHitResult _array_element)) (* (.Normal (Collision|BreakHitResult _array_element)) _sphereradius)) (* (Transformation|GetActorForwardVector) _sphereradius)) (.Normal (Collision|BreakHitResult _array_element)))
        (goto _label Break)))
    (:Completed
      (Utilities|FlowControl|Sequence
        (:then_0
          (Effects|SpawnEmitteratLocation "/Game/SciFiWeapLight/FX/Particles/P_Impact_Metal_Large_Light.P_Impact_Metal_Large_Light" (.Location (Collision|BreakHitResult _array_element)) (Math|Conversions|RotationFromXVector (Math|Vector|RotateVectorAroundAxis (.Normal (Collision|BreakHitResult _array_element)) (Math|Random|RandomFloatinRange -1.8e+02 1.8e+02) (.Normal (Collision|BreakHitResult _array_element))))))
        (:then_1
          (for _index (range 0 (- (Variables|Default|GetFrag%20Projectile%20Number) 1))
            (bind _returnvalue_2 (Class|TPSFunctionLibrary|CircleDistributionRandom (Variables|Default|GetFrag%20Spread) (Variables|Default|GetFrag%20Spread%20with%20Normal%20Distribution)))
            (bind _returnvalue_3 (Game|SpawnActorfromClass "/Game/_MyAssets/BP_Weapons/Projectiles/BP_Frag_Light_HEIAP.BP_Frag_Light_HEIAP_C" (Math|Transform|MakeTransform (+ (.Location (Collision|BreakHitResult _array_element)) (* (.Normal (Collision|BreakHitResult _array_element)) 5.0)) (Math|Rotator|MakeRotator _roll (+ _pitch (.X (Math|Vector2D|BreakVector2D _returnvalue_2))) (+ _yaw (.Y (Math|Vector2D|BreakVector2D _returnvalue_2)))) (Math|Conversions|ToVector(Float) (Variables|Default|GetFrag%20Projectile%20Scale))) "AlwaysSpawn" self (Variables|Default|GetInstigator)))
            (Utilities|FlowControl|Sequence
              (:then_0
                (bind _output_get (Variables|/Script/Engine.ProjectileMovementComponent|SetInitialSpeed (Variables|/Script/TPS.Projectile|GetProjectileMovementComponent _returnvalue_3) (Variables|Default|GetFrag%20Initial%20Velocity)))
                (Variables|/Script/Engine.ProjectileMovementComponent|SetMaxSpeed (Variables|/Script/TPS.Projectile|GetProjectileMovementComponent _returnvalue_3) _output_get))
              (:then_1
                (Variables|/Script/TPS.Projectile|SetRange _returnvalue_3 (Variables|Default|GetFrag%20Range)))
              (:then_2
                (Class|Projectile|FireinDirection _returnvalue_3 (Transformation|GetActorForwardVector _returnvalue_3)))))
          (Actor|DestroyActor))))))

(event EventBeginPlay
  (|CallParentFunction) ; 此节点被禁用，将不会被调用。\n从引脚连出引线来编译功能。
)

(event Collision|EventActorBeginOverlap
  (params (OtherActor :type Actor%20Object%20Reference))
  (|CallParentFunction OtherActor))

(event EventTick
  (params (DeltaSeconds :type Float%20%28single-precision%29))
  (|CallParentFunction DeltaSeconds) ; 此节点被禁用，将不会被调用。\n从引脚连出引线来编译功能。
)

(fn ConstructionScript
  (|CallParentFunction)
  (Variables|Default|SetHitEmitter "/Game/SciFiWeapLight/FX/Particles/P_Impact_Metal_Large_Light.P_Impact_Metal_Large_Light")
  (Variables|Default|SetHitSound "/Game/SciFiWeapLight/Sound/SniperRifle/SR_ImpactSurface_Cue.SR_ImpactSurface_Cue"))