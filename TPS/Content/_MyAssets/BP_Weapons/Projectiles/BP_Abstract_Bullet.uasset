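; Base bullet projectile that destroys itself once it travels beyond Range from StartLocation, or when it hits something.
; On hit it spawns an impact emitter, an attenuated sound and a bullet hole decal; it applies no damage itself.
; The decal projects along the bullet's forward vector with random roll, its depth scaled by the tangent of the impact angle.
; Unconnected line-trace and decal experiments remain in the EventGraph.
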(event EventBeginPlay)

(event Collision|EventActorBeginOverlap
  (params (OtherActor :type Actor%20Object%20Reference)))

(event EventTick
  (params (DeltaSeconds :type Float%20%28single-precision%29))
  (if (> (Math|Vector|VectorLength (- (Transformation|GetActorLocation) (Variables|Default|GetStartLocation))) (Variables|Default|GetRange))
    (Actor|DestroyActor)))

(event Collision|EventHit
  (params (MyComp :type Primitive%20Component%20Object%20Reference) (Other :type Actor%20Object%20Reference) (OtherComp :type Primitive%20Component%20Object%20Reference) (bSelfMoved :type Boolean) (HitLocation :type Vector :default "0, 0, 0") (HitNormal :type Vector :default "0, 0, 0") (NormalImpulse :type Vector :default "0, 0, 0") (Hit :type Hit%20Result%20Structure%20%28by%20ref%29))
  (bind _returnvalue (Math|Conversions|RotationFromXVector HitNormal))
  (bind _collider (Variables|Default|GetCollider))
  (bind _sphereradius (Variables|/Script/Engine.SphereComponent|GetSphereRadius _collider))
  (Utilities|FlowControl|Sequence
    (:then_0
      (Effects|SpawnEmitteratLocation (Variables|Default|GetHitEmitter) HitLocation _returnvalue (Math|Conversions|ToVector(Float) (Variables|Default|GetEmitterScale))))
    (:then_1
      (Audio|PlaySoundatLocation (Variables|Default|GetHitSound) HitLocation _returnvalue 1.0 1.0 0.0 (Variables|Default|GetHitSoundAttenuation) 0 0))
    (:then_2
      (CallFunction|SpawnBulletHoleDecal (+ (+ HitLocation (* HitNormal _sphereradius)) (* (Transformation|GetActorForwardVector) _sphereradius)) HitNormal))
    (:then_3
      (Actor|DestroyActor))))

(fn ConstructionScript
  (Variables|Default|SetHitSoundAttenuation "/Game/SciFiWeapLight/Sound/Attenuation/ProjectileImpact_att.ProjectileImpact_att"))

(fn SpawnBulletHoleDecal
  (params (Location :type Vector) (Normal :type Vector))
  (bind _bulletholesize (Variables|Default|GetBulletHoleSize))
  (bind _returnvalue (Rendering|Decal|SpawnDecalatLocation "/Game/_MyAssets/Materials/M_BulletHole.M_BulletHole" (Math|Vector|MakeVector (* (Math|Float|Absolute(Float) (Math|Trig|Tan(Degrees) (Class|KismetMathLibrary|DegAcos (Math|Vector|DotProduct (Math|Vector|Normalize Normal) (Math|Vector|Normalize (Transformation|GetActorForwardVector)))))) _bulletholesize) _bulletholesize _bulletholesize) Location (Math|Transform|TransformRotation (Math|Conversions|ToTransform(Rotator) (Math|Conversions|RotationFromXVector (Transformation|GetActorForwardVector))) (Math|Rotator|MakeRotator (Math|Random|RandomFloatinRange -1.8e+02 1.8e+02) 0.0 0.0)) 0.0))
  (Rendering|Components|Decal|SetFadeScreenSize _returnvalue 0.0)
  (return _returnvalue))