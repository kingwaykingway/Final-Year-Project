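; Base rocket projectile that homes toward a target location.
; Each Tick, with FireAndIgnore set, it refreshes that location from a valid LockedTarget's position.
; When its heading is off target, it interpolates the forward vector toward the target at RotationFlexibility speed and passes it to FireInDirection.
; The Hit event is empty; its emitter, sound and destroy logic is disconnected and never runs.
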(event EventBeginPlay)

(event Collision|EventActorBeginOverlap
  (params (OtherActor :type Actor%20Object%20Reference)))

(event EventTick
  (params (DeltaSeconds :type Float%20%28single-precision%29))
  (bind _lockedtarget (Variables|Default|GetLockedTarget))
  (bind _rootcomponent (Variables|Transformation|GetRootComponent))
  (bind _returnvalue (Math|Vector|GetForwardVector _rootcomponent))
  (Utilities|FlowControl|Sequence
    (:then_0
      (if (Variables|Default|GetFire%20and%20Ignore)
        (Utilities|IsValid _lockedtarget
          (:Is%20Valid
            (Variables|Default|SetTarget%20Location (Transformation|GetActorLocation _lockedtarget))))))
    (:then_1
      (bind _returnvalue_2 (Class|TPSFunctionLibrary|AngleBetweenVectors (- (Variables|Default|GetTarget%20Location) (Transformation|GetWorldLocation _rootcomponent)) _returnvalue))
      (if (!= _returnvalue_2 0.0)
        (Utilities|IsValid (Variables|Default|GetProjectileMovementComponent)
          (:Is%20Valid
            (Class|Projectile|FireinDirection (Math|Interpolation|VInterpTo (Math|Vector|Normalize _returnvalue) (Math|Vector|Normalize (- (Variables|Default|GetTarget%20Location) (Transformation|GetWorldLocation _rootcomponent))) DeltaSeconds (Variables|Default|GetRotation%20Flexibility)))))))))

(event Collision|EventHit
  (params (MyComp :type Primitive%20Component%20Object%20Reference) (Other :type Actor%20Object%20Reference) (OtherComp :type Primitive%20Component%20Object%20Reference) (bSelfMoved :type Boolean) (HitLocation :type Vector :default "0, 0, 0") (HitNormal :type Vector :default "0, 0, 0") (NormalImpulse :type Vector :default "0, 0, 0") (Hit :type Hit%20Result%20Structure%20%28by%20ref%29)))

(fn ConstructionScript)

(fn AngleBetweenVectors
  (params (HostVector :type Vector) (GuestVector :type Vector))
  (return (Class|KismetMathLibrary|DegAcos (Math|Vector|DotProduct (Math|Vector|Normalize HostVector) (Math|Vector|Normalize GuestVector)))))