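; BP_Missile_Light is a light missile projectile that explodes on impact.
; On Hit it spawns the light rocket explosion emitter, scaled by EmitterScale, and plays an attenuated explosion sound at the hit location, then destroys itself.
; The effect's rotation comes from the hit normal with pitch offset 90 degrees down, aligning the blast to the surface.
; The graph itself applies no damage.
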(event EventBeginPlay
  (|CallParentFunction) ; 此节点被禁用，将不会被调用。\n从引脚连出引线来编译功能。
)

(event Collision|EventActorBeginOverlap
  (params (OtherActor :type Actor%20Object%20Reference))
  (|CallParentFunction OtherActor) ; 此节点被禁用，将不会被调用。\n从引脚连出引线来编译功能。
)

(event EventTick
  (params (DeltaSeconds :type Float%20%28single-precision%29))
  (|CallParentFunction DeltaSeconds) ; 此节点被禁用，将不会被调用。\n从引脚连出引线来编译功能。
)

(event Collision|EventHit
  (params (MyComp :type Primitive%20Component%20Object%20Reference) (Other :type Actor%20Object%20Reference) (OtherComp :type Primitive%20Component%20Object%20Reference) (bSelfMoved :type Boolean) (HitLocation :type Vector :default "0, 0, 0") (HitNormal :type Vector :default "0, 0, 0") (NormalImpulse :type Vector :default "0, 0, 0") (Hit :type Hit%20Result%20Structure%20%28by%20ref%29))
  (bind _returnvalue (Math|Conversions|RotationFromXVector HitNormal))
  (bind (_roll _pitch _yaw) (Math|Rotator|BreakRotator _returnvalue))
  (bind _returnvalue_2 (- _pitch 9e+01))
  (bind _returnvalue_3 (Math|Rotator|MakeRotator _roll _returnvalue_2 _yaw))
  (Utilities|FlowControl|Sequence
    (:then_0
      (Effects|SpawnEmitteratLocation "/Game/SciFiWeapLight/FX/Particles/P_RocketLauncher_Explosion_Light.P_RocketLauncher_Explosion_Light" HitLocation _returnvalue_3 (Math|Conversions|ToVector(Float) (Variables|Default|GetEmitterScale))))
    (:then_1
      (Audio|PlaySoundatLocation "/Game/SciFiWeapLight/Sound/RocketLauncher/RL_Explosion_Cue.RL_Explosion_Cue" HitLocation _returnvalue_3 1.0 1.0 0.0 "/Game/SciFiWeapLight/Sound/Attenuation/Explosion_att.Explosion_att" 0 0))
    (:then_2
      (Actor|DestroyActor))))

(fn ConstructionScript
  (|CallParentFunction))