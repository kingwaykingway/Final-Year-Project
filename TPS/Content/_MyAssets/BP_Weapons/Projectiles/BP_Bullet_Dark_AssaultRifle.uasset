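; Dark-variant assault rifle bullet projectile that supplies its own impact effects to inherited projectile logic.
; The construction script calls the parent's, then sets HitEmitter to a dark medium metal impact particle and HitSound to a rifle surface impact cue.
; Its event graph runs nothing: the events are disabled, and a disconnected impact sequence of emitter, sound and destroy remains unused.
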(event EventBeginPlay
  (|CallParentFunction) ; 此节点被禁用，将不会被调用。\n从引脚连出引线来编译功能。
)

(event Collision|EventActorBeginOverlap
  (params (OtherActor :type Actor%20Object%20Reference))
  (|CallParentFunction OtherActor) ; 此节点被禁用，将不会被调用。\n从引脚连出引线来编译功能。
)

(event EventTick
  (params (DeltaSeconds :type Float%20%28single-precision%29))
  (|CallParentFunction DeltaSeconds) ; 此节点被禁用，将不会被调用。\n从引脚连出引线来编译功能。
)

(fn ConstructionScript
  (|CallParentFunction)
  (Variables|Default|SetHitEmitter "/Game/SciFiWeapDark/FX/Particles/P_Impact_Metal_Medium_Dark.P_Impact_Metal_Medium_Dark")
  (Variables|Default|SetHitSound "/Game/SciFiWeapDark/Sound/Rifle/Rifle_ImpactSurface_Cue.Rifle_ImpactSurface_Cue"))