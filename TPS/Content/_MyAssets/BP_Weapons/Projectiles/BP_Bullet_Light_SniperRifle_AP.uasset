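; Armor-piercing light sniper rifle bullet, a child projectile that marks where it enters and exits the surfaces it passes through.
; Collider begin overlap spawns the impact emitter, sound and bullet hole decal at the sweep hit.
; End overlap spawns an exit emitter, then line traces back toward StartLocation, with persistent debug drawing, to place the exit hole.
; The construction script sets metal impact effects; Tick prints distance from StartLocation once for debugging.
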(event OnComponentBeginOverlap(Collider)
  (params (OverlappedComponent :type Primitive%20Component%20Object%20Reference) (OtherActor :type Actor%20Object%20Reference) (OtherComp :type Primitive%20Component%20Object%20Reference) (OtherBodyIndex :type Integer) (bFromSweep :type Boolean) (SweepResult :type Hit%20Result%20Structure%20%28by%20ref%29))
  (bind (_bblockinghit _binitialoverlap _time _distance _location _impactpoint _normal) (Collision|BreakHitResult SweepResult))
  (bind _returnvalue (Math|Conversions|RotationFromXVector _normal))
  (Variables|Default|SetIs%20Overlapping true)
  (Utilities|FlowControl|Sequence
    (:then_0
      (Effects|SpawnEmitteratLocation (Variables|Default|GetHitEmitter) _location _returnvalue (Math|Conversions|ToVector(Float) (Variables|Default|GetEmitterScale))))
    (:then_1
      (Audio|PlaySoundatLocation (Variables|Default|GetHitSound) _location _returnvalue 1.0 1.0 0.0 (Variables|Default|GetHitSoundAttenuation) 0 0))
    (:then_2
      (CallFunction|SpawnBulletHoleDecal (+ _location (* (Transformation|GetActorForwardVector) (Variables|/Script/Engine.SphereComponent|GetSphereRadius (Variables|Default|GetCollider)))) _normal))))

(event OnComponentEndOverlap(Collider)
  (params (OverlappedComponent :type Primitive%20Component%20Object%20Reference) (OtherActor :type Actor%20Object%20Reference) (OtherComp :type Primitive%20Component%20Object%20Reference) (OtherBodyIndex :type Integer))
  (bind _returnvalue (Transformation|GetActorTransform))
  (bind (_location _rotation) (Math|Transform|BreakTransform _returnvalue))
  (Variables|Default|SetIs%20Overlapping false)
  (Utilities|FlowControl|Sequence
    (:then_0
      (Effects|SpawnEmitteratLocation "/Game/SciFiWeapLight/FX/Particles/P_Impact_Metal_Large_Light.P_Impact_Metal_Large_Light" _location _rotation))
    (:then_1
      (bind _outhit (Collision|LineTraceByChannel (Transformation|GetActorLocation) (Variables|Default|GetStartLocation) "TraceTypeQuery1" false 0 "Persistent"))
      (if (.bBlockingHit (Collision|BreakHitResult _outhit))
        (CallFunction|SpawnBulletHoleDecal (.Location (Collision|BreakHitResult _outhit)) (.Normal (Collision|BreakHitResult _outhit)))))))

(event EventBeginPlay
  (|CallParentFunction) ; 此节点被禁用，将不会被调用。\n从引脚连出引线来编译功能。
)

(event Collision|EventActorBeginOverlap
  (params (OtherActor :type Actor%20Object%20Reference))
  (|CallParentFunction OtherActor))

(event EventTick
  (params (DeltaSeconds :type Float%20%28single-precision%29))
  (|CallParentFunction DeltaSeconds)
  (Utilities|FlowControl|DoOnce false
    (:Completed
      (Development|PrintString (Utilities|String|ToString(Float) (Math|Vector|VectorLength (- (Transformation|GetActorLocation) (Variables|Default|GetStartLocation))))))))

(fn ConstructionScript
  (|CallParentFunction)
  (Variables|Default|SetHitEmitter "/Game/SciFiWeapLight/FX/Particles/P_Impact_Metal_Large_Light.P_Impact_Metal_Large_Light")
  (Variables|Default|SetHitSound "/Game/SciFiWeapLight/Sound/SniperRifle/SR_ImpactSurface_Cue.SR_ImpactSurface_Cue"))