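; Light assault rifle weapon Blueprint that supplies rifle-specific crosshair and reload visuals, apparently on top of a parent weapon class.
; Its child begin-play event sets the crosshair's sight pattern to a dot when the crosshair is valid.
; Separate hip, ironsights and prone reload events each play a matching non-looping animation on the gun mesh.
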(event EventBeginPlay)

(event Collision|EventActorBeginOverlap
  (params (OtherActor :type Actor%20Object%20Reference)))

(event EventTick
  (params (DeltaSeconds :type Float%20%28single-precision%29)))

(event EventReloadHip
  ;[1 1 1] Reloadings
  (Components|Animation|PlayAnimation (Variables|Default|GetGunMesh) "/Game/SciFiWeapLight/Weapons/Anims/Reload_Rifle_Hips_W.Reload_Rifle_Hips_W" false))

(event EventReloadProne
  ;[1 1 1] Reloadings
  (Components|Animation|PlayAnimation (Variables|Default|GetGunMesh) "/Game/SciFiWeapLight/Weapons/Anims/Prone_Reload_Rifle_W.Prone_Reload_Rifle_W" false))

(event EventReloadIronsights
  ;[1 1 1] Reloadings
  (Components|Animation|PlayAnimation (Variables|Default|GetGunMesh) "/Game/SciFiWeapLight/Weapons/Anims/Reload_Rifle_Ironsights_W.Reload_Rifle_Ironsights_w" false))

(event EventBeginPlayChild
  (bind _crosshair (Variables|Default|GetCrosshair))
  (Utilities|IsValid _crosshair
    (:Is%20Valid
      (Variables|/Script/TPS.CrosshairWidget|SetSightPattern _crosshair "SightPattern_Dot"))))

(fn ConstructionScript)