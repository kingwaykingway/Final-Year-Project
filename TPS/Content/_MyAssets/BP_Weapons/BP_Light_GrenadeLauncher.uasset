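; Light grenade launcher weapon Blueprint that handles firing, reloading and aiming.
; Fire plays an animation, decrements ammo and spawns a projectile from the muzzle offset, launched forward at muzzle velocity.
; All three reload stances share one animation, and the laser pointer shows the predicted projectile arc through one-frame debug drawing.
; Scope aiming blends the player's view to the weapon itself and switches back to the character on release.
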(event EventBeginPlay)

(event Collision|EventActorBeginOverlap
  (params (OtherActor :type Actor%20Object%20Reference)))

(event EventAimScope
  (params (activate :type Boolean))
  (bind _returnvalue (Game|GetPlayerController 0))
  ;[1 1 1] Override aiming down scope
  (if activate
    (Game|Player|SetViewTargetwithBlend _returnvalue self (Variables|Default|GetAimingDelay) "VTBlend_Linear" 0.0 false)
    (else
      (Game|Player|SetViewTargetwithBlend _returnvalue (Game|GetPlayerCharacter _returnvalue) 0.0 "VTBlend_Linear" 0.0 false))))

(event EventTick
  (params (DeltaSeconds :type Float%20%28single-precision%29)))

(event EventReloadHip
  ;[1 1 1] Reloadings
  (Components|Animation|PlayAnimation (Variables|Default|GetSkeletalMesh) "/Game/SciFiWeapLight/Weapons/Anims/Reload_GrenadeLauncher_W.Reload_GrenadeLauncher_W" false))

(event EventFire
  ;[1 1 1] Fire
  (Components|Animation|PlayAnimation (Variables|Default|GetSkeletalMesh) "/Game/SciFiWeapLight/Weapons/Anims/Fire_GrenadeLauncher_W.Fire_GrenadeLauncher_W" false)
  (Variables|Default|SetRemainingAmmo (- (Variables|Default|GetRemainingAmmo) 1))
  (bind _returnvalue (Game|SpawnActorfromClass (Variables|Default|GetProjectileClass) (Math|Transform|MakeTransform (+ (Transformation|GetActorLocation) (Math|Transform|TransformLocation (Math|Conversions|ToTransform(Rotator) (Transformation|GetActorRotation)) (Variables|Default|GetMuzzleOffset))) (Transformation|GetActorRotation) (Math|Conversions|ToVector(Float) (Variables|Default|GetProjectileScale))) "AlwaysSpawn" self (Variables|Default|GetInstigator)))
  (Utilities|FlowControl|Sequence
    (:then_0
      (bind _output_get (Variables|/Script/Engine.ProjectileMovementComponent|SetInitialSpeed (Variables|/Script/TPS.Projectile|GetProjectileMovementComponent _returnvalue) (Variables|Default|GetMuzzleVelocity)))
      (Variables|/Script/Engine.ProjectileMovementComponent|SetMaxSpeed (Variables|/Script/TPS.Projectile|GetProjectileMovementComponent _returnvalue) _output_get))
    (:then_1
      (Class|Projectile|FireinDirection _returnvalue (Transformation|GetActorForwardVector _returnvalue)))))

(event EventReloadProne
  ;[1 1 1] Reloadings
  (Components|Animation|PlayAnimation (Variables|Default|GetSkeletalMesh) "/Game/SciFiWeapLight/Weapons/Anims/Reload_GrenadeLauncher_W.Reload_GrenadeLauncher_W" false))

(event EventReloadIronsights
  ;[1 1 1] Reloadings
  (Components|Animation|PlayAnimation (Variables|Default|GetSkeletalMesh) "/Game/SciFiWeapLight/Weapons/Anims/Reload_GrenadeLauncher_W.Reload_GrenadeLauncher_W" false))

(event EventAimLazerPointer
  (params (activate :type Boolean))
  (bind _lazer_pointer (Variables|Default|GetLazer%20Pointer))
  (Class|GameplayStatics|BlueprintPredictProjectilePathbyTraceChannel (Transformation|GetWorldLocation _lazer_pointer) (* (Math|Vector|GetForwardVector _lazer_pointer) (Variables|Default|GetMuzzleVelocity)) true 0.0 "ECC_WorldDynamic" false 0 "ForOneFrame"))

(fn ConstructionScript)